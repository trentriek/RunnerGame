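; BPC_Timer is a Blueprint component that tracks elapsed play time in whole seconds.
; StartTimer runs a looping one-second function timer instead of Tick, trading precision for performance, and StopTimer clears its handle.
; Each update increments TotalSeconds and fires the TimerAddedSecond dispatcher for listeners.
; ReturnTotalTime splits the running total into hours, minutes and seconds.
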(event `Start Timer`
  ;[1 1 1] For the Timer we will use a timer node, and update every second. This will be better for performance and have a more constant value, since it doesn't matter the exact time just that the player finished before times up.
  ;
  ; IF we were creating PVP, a precise time would be desired and the functionality would be moved to a tick function.
  (bind _returnvalue (`KismetSystemLibrary.K2_SetTimer` null "TimerUpdate" 1.0 true))
  (set `self.TimerHandle` _returnvalue))

(event `Stop Timer`
  ;[1 1 1] For the Timer we will use a timer node, and update every second. This will be better for performance and have a more constant value, since it doesn't matter the exact time just that the player finished before times up.
  ;
  ; IF we were creating PVP, a precise time would be desired and the functionality would be moved to a tick function.
  (`KismetSystemLibrary.K2_ClearAndInvalidateTimerHandle` (`self.TimerHandle`)))

(fn `ReturnTotalTime`
  (returns (Hours :type Integer) (Minutes :type Integer) (Seconds :type Integer))
  (bind _totalseconds (`self.TotalSeconds`))
  (bind _returnvalue (/ _totalseconds 60))
  (return (/ _returnvalue 60) (mod _returnvalue 60) (mod _totalseconds 60)))

(fn `TimerUpdate`
  (`/Engine/EditorBlueprintResources/StandardMacros.IncrementInt` (`self.TotalSeconds`)
    (:`  `
      (`self.TimerAddedSecond`))))