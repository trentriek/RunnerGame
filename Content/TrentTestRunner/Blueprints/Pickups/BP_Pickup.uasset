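; BP_Pickup is a collectible actor that reports to the game's pickup manager when an actor overlaps its sphere.
; The first overlap clears CanBeCollected to block repeat collection, then passes the pickup and overlapping actor to BPC_PickupManager on the GameState.
; A debug string prints on collection.
; Unconnected Niagara nodes remain from an unfinished attempt to change the effect's mesh from Blueprint.
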(event `self.Sphere.OnComponentBeginOverlap`
  (params (OverlappedComponent :type "PrimitiveComponent Object Reference") (OtherActor :type "Actor Object Reference") (OtherComp :type "PrimitiveComponent Object Reference") (OtherBodyIndex :type Integer) (bFromSweep :type Boolean) (SweepResult :type "HitResult Structure (by ref)"))
  (if (`self.CanBeCollected`)
    (set `self.CanBeCollected` false)
    (`/Game/TrentTestRunner/Blueprints/BPC_PickupManager.PickupCollected` (`self.GetComponentByClass` (`GameplayStatics.GetGameState`) "/Game/TrentTestRunner/Blueprints/BPC_PickupManager.BPC_PickupManager_C") self OtherActor)
    (`KismetSystemLibrary.PrintString` "Pickup!")))

(fn `UserConstructionScript`)