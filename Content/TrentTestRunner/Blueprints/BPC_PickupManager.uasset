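; BPC_PickupManager is a component that owns the lifecycle of all BP_Pickup actors, tracking them in the PickupObjects array.
; It gathers level-placed pickups on BeginPlay and spawns new ones from a pickup struct and transform.
; On collection it forwards the pickup struct to the capturing actor via CollectPickupMessage, leaving the effect to that actor, then untracks and destroys the pickup.
; The array's RepNotify prints the pickup count for debugging.
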(event `self.ReceiveBeginPlay`
  ;[1 1 1] Collect any pickups placed at the beginning.
  (bind _outactors (`GameplayStatics.GetAllActorsOfClass` "/Game/TrentTestRunner/Blueprints/Pickups/BP_Pickup.BP_Pickup_C"))
  (`KismetArrayLibrary.Array_Append` (`self.PickupObjects`) _outactors))

(event `PickupCollected`
  (params (`Pickup reference` :type "/Game/TrentTestRunner/Blueprints/Pickups/BP_Pickup Object Reference") (`Actor that captured pickup` :type "Actor Object Reference"))
  (message `/Game/TrentTestRunner/Blueprints/Pickups/BPI_PickupCalls.CollectPickup` `Actor that captured pickup` (`/Game/TrentTestRunner/Blueprints/Pickups/BP_Pickup.Pickup Struct` `Pickup reference`)) ; The Pickup Manager should handle all instances of the pickups.\nIt will forward the pickup data to actor which will handle the what\nhappens during the pickup.
  (`KismetArrayLibrary.Array_RemoveItem` (`self.PickupObjects`) `Pickup reference`)
  (`self.DestroyPickup` `Pickup reference`))

(event `DestroyPickup`
  (params (`Pickup Ref` :type "/Game/TrentTestRunner/Blueprints/Pickups/BP_Pickup Object Reference"))
  (`Actor.K2_DestroyActor` `Pickup Ref`))

(event `PickupSpawn`
  (params (`Pickup Struct` :type "/Game/TrentTestRunner/Blueprints/Pickups/ST_Pickup Structure") (`Pickup Transform` :type "Transform Structure"))
  (bind _returnvalue (`|SpawnActorFromClass` "/Game/TrentTestRunner/Blueprints/Pickups/BP_Pickup.BP_Pickup_C" `Pickup Transform` "Undefined" "OverrideRootScale" null `Pickup Struct` null))
  (`KismetArrayLibrary.Array_Add` (`self.PickupObjects`) _returnvalue))

(fn `OnRep_PickupObjects`
  (`KismetSystemLibrary.PrintString` (`KismetStringLibrary.Concat_StrStr` "# of pickups: " (`KismetStringLibrary.Conv_IntToString` (`KismetArrayLibrary.Array_Length` (`self.PickupObjects`))))) ; Left here to test to make sure the array is updating
)