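; Player controller for the runner game that sets up the player UI and manages score and game-over state.
; On BeginPlay it adds WBP_PlayerUI and binds the timer component's time-limit event to a loss.
; Failure records the result in BP_Runner_PlayerState, fires the game-over dispatcher and spawns a spectator pawn, which the server possesses after destroying the runner.
; UpdateScore adds points to the player state and broadcasts the change.
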(event `self.ReceiveBeginPlay`
  ;[1 1 1] Begin Play - add widget to viewport
  (`/Engine/EditorBlueprintResources/ActorMacros.Switch Has Authority` ; @TODO: The remote connection throws errors in Multiplayer but is essential for singleplayer currently. \nNeed to find better way to check for singleplayer
    (:`Authority`
      _)
    (:`Remote`
      _))
  (bind _returnvalue (`|CreateWidget` "/Game/TrentTestRunner/Widgets/WBP_PlayerUI.WBP_PlayerUI_C" self))
  (`UserWidget.AddToViewport` _returnvalue 0)
  ;[1 1 1] Handle Player game Over upon Timer Complete
  (add `/Game/TrentTestRunner/Blueprints/Timer/BPC_Timer.TimeLimitReached` (`self.BPC_Timer`) (delegate `GameFailed`)))

(event `GameFailed`
  ;[1 1 1] Handle Player game Over upon Timer Complete
  (`self.GameOver` false)
  (`self.SetPawn`))

(event `GameOver`
  (params (Win :type Boolean))
  ;[1 1 1] Comment
  (bind _asbp_runner_player_state (cast `/Game/TrentTestRunner/Base/BP_Runner_PlayerState` (`self.PlayerState`)))
  (bind _output_get (set `/Game/TrentTestRunner/Base/BP_Runner_PlayerState.PlayerWin` Win _asbp_runner_player_state))
  (`self.PlayerGameOver` _output_get))

(event `SetPawn`
  (bind _returnvalue (`self.K2_GetPawn`))
  ;[1 1 1] Handle Player game Over upon Timer Complete
  (bind _returnvalue_2 (`|SpawnActorFromClass` "/Script/Engine.SpectatorPawn" (`self.GetTransform` _returnvalue) "Undefined" "OverrideRootScale" null null))
  (`/Engine/EditorBlueprintResources/ActorMacros.Switch Has Authority`
    (:`Authority`
      (`self.K2_DestroyActor` _returnvalue)
      (`self.Possess` _returnvalue_2))))

(event `UpdateScore`
  (params (ScoreNum :type Integer))
  ;[1 1 1] Comment
  (bind _asbp_runner_player_state (cast `/Game/TrentTestRunner/Base/BP_Runner_PlayerState` (`self.PlayerState`)))
  (set `/Game/TrentTestRunner/Base/BP_Runner_PlayerState.RunnerScore` (+ (`/Game/TrentTestRunner/Base/BP_Runner_PlayerState.RunnerScore` _asbp_runner_player_state) ScoreNum) _asbp_runner_player_state)
  (`self.ScoreUpdated`))

(fn `UserConstructionScript`)